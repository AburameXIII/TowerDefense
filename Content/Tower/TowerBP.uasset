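; Tower actor for a tower-defense-style game that automatically targets and shoots Runners within its range.
; On BeginPlay, TowerData sets its mesh, material, range sphere and range plane scale.
; Each Tick it faces and fires projectiles with effects at its target, gated by a fire-rate cooldown.
; Without a target, a throttled sphere trace picks the closest Runner, and the target clears on leaving the range sphere.
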(event `self.ReceiveBeginPlay`
  (`self.TowerInitialization`))

(event `Shoot`
  (bind _returnvalue (`self.K2_GetActorLocation`))
  (bind (_name _damage _range _projectilespeed _firerate _cost _mesh _material _shootingparticle _shootingsound) (break `/Game/Tower/TowerData` (`self.TowerData`)))
  ;[1 1 1] Shoots a projectile to the current target
  (set `self.Cooldown` true)
  (`|SpawnActorFromClass` "/Game/Tower/Projectile.Projectile_C" (`self.GetTransform`) "AlwaysSpawn" "OverrideRootScale" null (`self.TowerTarget`) _projectilespeed _damage _range _returnvalue null)
  (`GameplayStatics.SpawnEmitterAtLocation` _shootingparticle _returnvalue)
  (`GameplayStatics.SpawnSoundAtLocation` _shootingsound _returnvalue (struct) 1.0 1.0 0.0 null null)
  (`KismetSystemLibrary.Delay` _firerate)
  (set `self.Cooldown` false))

(event `TowerInitialization`
  (bind _towermesh (`self.TowerMesh`))
  (bind _plane (`self.Plane`))
  (bind (_name _damage _range _projectilespeed _firerate _cost _mesh _material) (break `/Game/Tower/TowerData` (`self.TowerData`)))
  ;[1 1 1] Initializes the tower parameters according to the data
  (`StaticMeshComponent.SetStaticMesh` _towermesh _mesh)
  (`PrimitiveComponent.SetMaterial` _towermesh 0 _material)
  (`SphereComponent.SetSphereRadius` (`self.Range`) _range true)
  (`SceneComponent.SetRelativeScale3D` _plane (* (`SceneComponent.RelativeScale3D` _plane) _range)))

(event `self.Range.OnComponentEndOverlap`
  (params (OverlappedComponent :type "PrimitiveComponent Object Reference") (OtherActor :type "Actor Object Reference") (OtherComp :type "PrimitiveComponent Object Reference") (OtherBodyIndex :type Integer))
  ;[1 1 1] If current target gets off range, lose target
  (if (== OtherActor (`self.TowerTarget`))
    (set `self.TowerTarget` null)))

(event `GetNewTarget`
  (bind _returnvalue (`self.K2_GetActorLocation`))
  ;[1 1 1] Responsible for finding a new target when the tower has no target
  (set `self.FindingNewTarget` true)
  (bind (_outhits _returnvalue_2) (`KismetSystemLibrary.SphereTraceMultiForObjects` _returnvalue (+ _returnvalue (0.0 0.0 0.1)) (`.Range_7_1104581B49E50BFFB13410A18092AC32` (break `/Game/Tower/TowerData` (`self.TowerData`))) (`|MakeArray` "ObjectTypeQuery3" :!type "EObjectTypeQuery Enum")))
  (if _returnvalue_2
    (bind _closesttarget (`self.ClosestTarget` _outhits))
    (`/Engine/EditorBlueprintResources/StandardMacros.IsValid` _closesttarget
      (:`Is Valid`
        (set `self.TowerTarget` _closesttarget))
      (:`Is Not Valid`
        _)))
  (`KismetSystemLibrary.Delay` 0.1)
  (set `self.FindingNewTarget` false))

(event `SetRotation`
  ;[1 1 1] Look at the Runner he is shooting at
  (`self.K2_SetActorRotation` (`KismetMathLibrary.FindLookAtRotation` (`self.K2_GetActorLocation`) (`self.K2_GetActorLocation` (`self.TowerTarget`)))))

(event `self.ReceiveTick`
  (params (DeltaSeconds :type "Float (single-precision)"))
  ;[1 1 1] Every tick, if it has a target, tries to shoot it, if not, tries to find a new one
  (`/Engine/EditorBlueprintResources/StandardMacros.IsValid` (`self.TowerTarget`)
    (:`Is Valid`
      (`self.SetRotation`)
      (if (not (`self.Cooldown`))
        (`self.Shoot`)))
    (:`Is Not Valid`
      (if (not (`self.FindingNewTarget`))
        (`self.GetNewTarget`)))))

(fn `ClosestTarget`
  (params (HitResults :type "Array of HitResult Structure"))
  (returns (ClosestTarget :type "/Game/Runner/Runner Object Reference"))
  (locals (TargetAux :type "/Game/Runner/Runner Object Reference") (Distance :type "Float (double-precision)"))
  (for _array_element HitResults
    (bind (_bblockinghit _binitialoverlap _time _distance _location _impactpoint _normal _impactnormal _physmat _hitactor) (`GameplayStatics.BreakHitResult` _array_element))
    (bind _asrunner (cast `/Game/Runner/Runner` _hitactor))
    (`/Engine/EditorBlueprintResources/StandardMacros.IsValid` (`local.TargetAux`)
      (:`Is Valid`
        (bind _returnvalue (`KismetMathLibrary.VSize` (- (`self.K2_GetActorLocation`) (`self.K2_GetActorLocation` _hitactor))))
        (if (< _returnvalue (`local.Distance`))
          (set `local.TargetAux` _asrunner)
          (set `local.Distance` _returnvalue)))
      (:`Is Not Valid`
        (set `local.TargetAux` _asrunner)
        (set `local.Distance` _returnvalue))))
  (return (`local.TargetAux`)))

(fn `UserConstructionScript`)