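; Placement preview actor for a tower in a tower defense game, showing the selected tower's mesh and a range circle scaled from its TowerData.
; Each tick it traces under the cursor, snaps to a grid at fixed height, and turns red over an existing tower or blue when valid.
; PlaceTower, when the spot is valid, spawns a TowerBP with that data, deducts its cost through the game mode and destroys the ghost.
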(event `self.ReceiveBeginPlay`
  (bind _plane (`self.Plane`))
  (bind (_name _damage _range _projectilespeed _firerate _cost _mesh) (break `/Game/Tower/TowerData` (`self.TowerData`)))
  ;[1 1 1] Set the right mesh for the right tower
  (`StaticMeshComponent.SetStaticMesh` (`self.GhostMesh`) _mesh)
  (`SceneComponent.SetRelativeScale3D` _plane (* (`SceneComponent.RelativeScale3D` _plane) _range)))

(event `self.ReceiveTick`
  (params (DeltaSeconds :type "Float (single-precision)"))
  (bind _ghostmesh (`self.GhostMesh`))
  (bind _plane (`self.Plane`))
  (bind (_hitresult _returnvalue) (`PlayerController.GetHitResultUnderCursorForObjects` (`GameplayStatics.GetPlayerController` 0) (`|MakeArray` "ObjectTypeQuery2" :!type "EObjectTypeQuery Enum") true))
  (bind (_bblockinghit _binitialoverlap _time _distance _location _impactpoint _normal _impactnormal _physmat _hitactor) (`GameplayStatics.BreakHitResult` _hitresult))
  ;[1 1 1] Follows Mouse Position and shows ghost on map
  (if _returnvalue
    (cast `/Game/Tower/TowerBP` _hitactor
      (:`then`
        (set `self.ValidPosition` false)
        (`PrimitiveComponent.SetMaterial` _ghostmesh 0 "/Game/Materials/GhostRedMaterial.GhostRedMaterial")
        (`PrimitiveComponent.SetMaterial` _plane 0 "/Game/Materials/CircleRed.CircleRed"))
      (:`CastFailed`
        (set `self.ValidPosition` true)
        (`PrimitiveComponent.SetMaterial` _ghostmesh 0 "/Game/Materials/GhostBlueMaterial.GhostBlueMaterial")
        (`PrimitiveComponent.SetMaterial` _plane 0 "/Game/Materials/Circle.Circle")))
    (`self.K2_SetActorLocation` (`KismetMathLibrary.MakeVector` (`KismetMathLibrary.GridSnap_Float` (.x _location) 150.0) (`KismetMathLibrary.GridSnap_Float` (.y _location) 150.0) 70.0))))

(event `Place Tower`
  (bind _towerdata (`self.TowerData`))
  ;[1 1 1] Places Tower
  (if (`self.ValidPosition`)
    (`|SpawnActorFromClass` "/Game/Tower/TowerBP.TowerBP_C" (`self.GetTransform`) "Undefined" "OverrideRootScale" null _towerdata null)
    (bind _astower_defense_game_mode (cast `/Game/GameLogic/TowerDefenseGameMode` (`GameplayStatics.GetGameMode`)))
    (`/Game/GameLogic/TowerDefenseGameMode.ChangeMoney` _astower_defense_game_mode (- 0 (`.Cost_22_DB9E5EE14EF2F268764AB8818F70B018` (break `/Game/Tower/TowerData` _towerdata))))
    (`self.K2_DestroyActor`)))

(fn `UserConstructionScript`)